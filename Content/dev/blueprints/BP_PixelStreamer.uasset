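; BP_PixelStreamer is an actor that bridges a Pixel Streaming web frontend and the game's configurator.
; On BeginPlay it finds the PixelStreamerInputComponent on the first player controller and binds its input event.
; Incoming descriptors are converted to JSON objects and passed to the BPConfigurator on BP_GameState as commands.
; SendMessageToFrontend returns data to the frontend as a Pixel Streaming response through the same component.
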(event Custom|UI%20Interaction
  (params (Descriptor :type String))
  (bind _output_get (Variables|Default|Setdescriptor Descriptor))
  (bind _asbp_game_state (Utilities|Casting|CastToBP_GameState (Game|GetGameState)))
  (Default|OnReceiveCommand (Variables|/Game/dev/blueprints/BP_GameState.BP_GameState_C|GetBP_Configurator _asbp_game_state) (Class|BlueprintJsonLibrary|ToJsonObject(String) _output_get)))

(event EventBeginPlay
  (bind _output_get (Variables|Default|SetPixelStreamerInput (Actor|GetComponentbyClass (Game|GetPlayerController 0) "/Script/PixelStreaming.PixelStreamerInputComponent")))
  (EventDispatchers|BindEventtoOnInputEvent _output_get (delegate Custom|UI%20Interaction)))

(fn ConstructionScript)

(fn SendMessagetoFrontend
  (params (data :type String))
  (Class|PixelStreamerInputComponent|SendPixelStreamingResponse (Variables|Default|GetPixelStreamerInput) data))