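; Player controller for a runtime transform-gizmo editor, handling mouse selection of objects and gizmo switching.
; Input actions set gizmo type and transformation space in BP_GameState, then broadcast the change to every BP_SelectableObject.
; Left click traces for a GizmoBase to start drag tracking, otherwise selects an ISelectable under the cursor or clears selection.
; Releasing the button ends tracking on all gizmos.
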(event EventBeginPlay
  ;[1 1 1] initial
  (Variables|Default|SetbShowMouseCursor true)
  (bind _asbp_game_state (Utilities|Casting|CastToBP_GameState (Game|GetGameState)))
  (Variables|Default|SetGameState _asbp_game_state))

(event EventEndPlay
  (params (EndPlayReason :type EEndPlayReason%20Enum :default "Destroyed"))
  ;[1 1 1] initial
  (Utilities|Time|ClearandInvalidateTimerbyHandle (Variables|Default|GetHoverCheckHandle)))

(event Input|ActionEvents|InputActionEnableRotationGizmo
  (params (Key :type Key%20Structure :default "None"))
  ;[1 1 1] handle gizmo type changed
  (:Pressed
    (CallFunction|GizmoTypeChanged "NewEnumerator1")))

(event Input|ActionEvents|InputActionEnableTranslationGizmo
  (params (Key :type Key%20Structure :default "None"))
  ;[1 1 1] handle gizmo type changed
  (:Pressed
    (CallFunction|GizmoTypeChanged "NewEnumerator0")))

(event Input|ActionEvents|InputActionEnableScaleGizmo
  (params (Key :type Key%20Structure :default "None"))
  ;[1 1 1] handle gizmo type changed
  (:Pressed
    (CallFunction|GizmoTypeChanged "NewEnumerator2")))

(event Input|ActionEvents|InputActionChangeTransformationSpace
  (params (Key :type Key%20Structure :default "None"))
  ;[1 1 1] transform space changed
  (:Pressed
    (CallFunction|TransformationSpaceChanged (select (Utilities|Enum|Equal(Enum) (.transformationspace (Variables|/Game/dev/blueprints/BP_GameState.BP_GameState_C|GetTransformation (Variables|Default|GetGameState))) "NewEnumerator0") "NewEnumerator1" "NewEnumerator0"))))

(event Input|MouseEvents|LeftMouseButton
  (params (Key :type Key%20Structure :default "None"))
  (bind (_hitresult _returnvalue) (Game|Player|GetHitResultUnderCursorbyChannel "TraceTypeQuery3" true))
  (bind _array (Utilities|Array|MakeArray "ObjectTypeQuery7"))
  (bind (_hitresult_2 _returnvalue_2) (Class|PlayerController|GetHitResultUnderCursorforObjects _array true))
  (bind _hitactor (Collision|BreakHitResult _hitresult_2))
  (:Pressed
    (CallFunction|ClearHoverState)
    ;[1 1 1] check if we click on gizmo
    (if _returnvalue
      (bind _asgizmo_base (Utilities|Casting|CastToGizmoBase (.HitActor (Collision|BreakHitResult _hitresult)))
        (:then
          (bind _returnvalue_3 (Class|GizmoBase|StartTracking _asgizmo_base))
          (|SetBy-RefVar (.bgizmodragging (Variables|/Game/dev/blueprints/BP_GameState.BP_GameState_C|GetTransformation (Variables|Default|GetGameState))) _returnvalue_3))
        (:CastFailed
          ;[1 1 1] if clicken on Selectable object
          (if _returnvalue_2 :!label _label
            (if (Utilities|DoesObjectImplementInterface _hitactor "/Game/dev/blueprints/ISelectable.ISelectable_C")
              (CallFunction|ClearSelection)
              (Class|ISelectable|SetSelected(Message) _hitactor true))
            (else
              (CallFunction|ClearSelection)))))
      (else
        (goto _label))))
  (:Released
    (CallFunction|SetGizmoTrackingEnabled false)))

(fn ConstructionScript)

(fn ClearHoverState
  (bind _outactors (Actor|GetAllActorsOfClass "/Game/dev/blueprints/BP_SelectableObject.BP_SelectableObject_C"))
  (for _array_element _outactors
    (Default|HoverLeave _array_element)))

(fn SetGizmoTrackingEnabled
  (params (EnableTracking :type Boolean))
  (bind _gamestate (Variables|Default|GetGameState))
  (bind _transformation (Variables|/Game/dev/blueprints/BP_GameState.BP_GameState_C|GetTransformation _gamestate))
  (|SetBy-RefVar (.bgizmodragging _transformation) EnableTracking)
  (bind _outactors (Actor|GetAllActorsOfClass "/Script/TransformToolRuntime.GizmoBase"))
  (for _array_element _outactors
    (if (.bgizmodragging _transformation)
      (Class|GizmoBase|StartTracking _array_element)
      (else
        (Class|GizmoBase|EndTracking _array_element)))))

(fn ClearSelection
  (bind _outactors (Actor|GetAllActorsOfClass "/Game/dev/blueprints/BP_SelectableObject.BP_SelectableObject_C"))
  (for _array_element _outactors
    (Class|ISelectable|SetSelected(Message) _array_element false)
    (Variables|Default|SetcurrentSelected 0)))

(fn GizmoTypeChanged
  (params (NewGizmo :type EGizmoType%20Enum :default "NewEnumerator0"))
  (bind _gamestate (Variables|Default|GetGameState))
  (bind _transformation (Variables|/Game/dev/blueprints/BP_GameState.BP_GameState_C|GetTransformation _gamestate))
  (|SetBy-RefVar (.currentgizmotype _transformation) NewGizmo)
  (bind _outactors (Actor|GetAllActorsOfClass "/Game/dev/blueprints/BP_SelectableObject.BP_SelectableObject_C"))
  (for _array_element _outactors
    (Class|ISelectable|GizmoTypeChanged(Message) _array_element (.currentgizmotype _transformation))))

(fn TransformationSpaceChanged
  (params (NewSpace :type ETransformationSpace%20Enum :default "NewEnumerator0"))
  (bind _gamestate (Variables|Default|GetGameState))
  (bind _transformation (Variables|/Game/dev/blueprints/BP_GameState.BP_GameState_C|GetTransformation _gamestate))
  (|SetBy-RefVar (.transformationspace _transformation) NewSpace)
  (bind _outactors (Actor|GetAllActorsOfClass "/Game/dev/blueprints/BP_SelectableObject.BP_SelectableObject_C"))
  (for _array_element _outactors
    (Class|IMovable|TransformationSpaceChanged(Message) _array_element (.transformationspace _transformation))))