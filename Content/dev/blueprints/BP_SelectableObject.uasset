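; BP_SelectableObject is an actor that can be selected and then moved, rotated or scaled with transform gizmos.
; SetSelected and GizmoTypeChanged spawn a translation, rotation or scale gizmo using the GameState's transformation space and bind its delta event.
; Translation deltas apply in world or local space, rotation always in world space, and scale only while X stays within limits.
; IsHovered and IsSelected are stubs returning false.
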(event Custom|SpawnGizmo
  (params (GizmoType :type EGizmoType%20Enum :default "NewEnumerator0"))
  (bind _self self)
  (bind _gamestate (Variables|Default|GetGameState))
  (bind _transformation (Variables|/Game/dev/blueprints/BP_GameState.BP_GameState_C|GetTransformation _gamestate))
  (bind _transformationspace (Utilities|Struct|BreakTransformState _transformation))
  (bind _result (CallFunction|GetInitialTransformforGizmo _transformationspace _self))
  ;[1 1 1] spawn gizmo
  (bind _output_get (Variables|Gizmo|SetselectedGizmoType GizmoType))
  (switch Utilities|FlowControl|Switch|SwitchonEGizmoType _output_get
    (:NewEnumerator0
      (bind _returnvalue (Game|SpawnActorfromClass "/Game/dev/blueprints/Gizmos/BP_TranslationGizmo.BP_TranslationGizmo_C" _result "AlwaysSpawn" 0 0))
      (bind _output_get_2 (Variables|Gizmo|SettrnaslationGizmo _returnvalue))
      (Variables|Gizmo|SetcurrentGizmo _output_get_2)
      (EventDispatchers|BindEventtoOnDeltaReceived _output_get_2 (EventDispatchers|CreateEvent :!event TranslationDeltaReceived)))
    (:NewEnumerator1
      (bind _returnvalue_2 (Game|SpawnActorfromClass "/Game/dev/blueprints/Gizmos/BP_RotationGizmo.BP_RotationGizmo_C" _result "AlwaysSpawn" 0 0))
      (bind _output_get_3 (Variables|Gizmo|SetrotationGizmo _returnvalue_2))
      (Variables|Gizmo|SetcurrentGizmo _output_get_3)
      (EventDispatchers|BindEventtoOnDeltaReceived _output_get_3 (EventDispatchers|CreateEvent :!event RotationDeltaReceived)))
    (:NewEnumerator2
      (bind _returnvalue_3 (Game|SpawnActorfromClass "/Game/dev/blueprints/Gizmos/BP_ScaleGizmo.BP_ScaleGizmo_C" _result "AlwaysSpawn" 0 0))
      (bind _output_get_4 (Variables|Gizmo|SetscaleGizmo _returnvalue_3))
      (Variables|Gizmo|SetcurrentGizmo _output_get_4)
      (EventDispatchers|BindEventtoOnDeltaReceived _output_get_4 (EventDispatchers|CreateEvent :!event ScaleDeltaReceived)))))

(event Custom|Event%20GizmoTypeChanged
  (params (new%20gizmo%20type :type EGizmoType%20Enum :default "NewEnumerator0"))
  ;[1 1 1] gizmo type changed
  (if (Variables|Default|GetbSelected)
    (Utilities|FlowControl|Sequence
      (:then_0
        (switch Utilities|FlowControl|Switch|SwitchonEGizmoType (Variables|Gizmo|GetselectedGizmoType)
          (:NewEnumerator0
            (EventDispatchers|UnbindallEventsfromOnDeltaReceived (Variables|Gizmo|GettrnaslationGizmo))
            (Actor|DestroyActor (Variables|Gizmo|GettrnaslationGizmo))
            (Variables|Gizmo|SettrnaslationGizmo 0))))
      (:then_1
        (Variables|Gizmo|SetcurrentGizmo 0)
        (EventDispatchers|UnbindallEventsfromOnDeltaReceived (Variables|Gizmo|GetrotationGizmo))
        (Actor|DestroyActor (Variables|Gizmo|GetrotationGizmo))
        (Variables|Gizmo|SetrotationGizmo 0))
      (:then_2
        (CallFunction|SpawnGizmo new%20gizmo%20type)
        (EventDispatchers|UnbindallEventsfromOnDeltaReceived (Variables|Gizmo|GetscaleGizmo))
        (Actor|DestroyActor (Variables|Gizmo|GetscaleGizmo))
        (Variables|Gizmo|SetscaleGizmo 0)))))

(event EventBeginPlay
  ;[1 1 1] init
  (bind _asbp_game_state (Utilities|Casting|CastToBP_GameState (Game|GetGameState)))
  (Variables|Default|SetGameState _asbp_game_state))

(event EventSetSelected
  (params (bSelected :type Boolean))
  ;[1 1 1] on selecting
  (Variables|Default|SetbSelected bSelected)
  (if true
    (CallFunction|HoverLeave)
    (CallFunction|SpawnGizmo (.CurrentGizmoType (Utilities|Struct|BreakTransformState (Variables|/Game/dev/blueprints/BP_GameState.BP_GameState_C|GetTransformation (Variables|Default|GetGameState)))))
    (else
      (bind _currentgizmo (Variables|Gizmo|GetcurrentGizmo)
        (:then
          (Actor|DestroyActor _currentgizmo)
          (Variables|Gizmo|SetcurrentGizmo 0))
        (:else)))))

(fn ConstructionScript)

(fn TranslationDeltaReceived
  (params (translationDelta :type Vector))
  (switch Utilities|FlowControl|Switch|SwitchonETransformationSpace (.TransformationSpace (Utilities|Struct|BreakTransformState (Variables|/Game/dev/blueprints/BP_GameState.BP_GameState_C|GetTransformation (Variables|Default|GetGameState))))
    (:NewEnumerator0
      (Transformation|AddActorWorldOffset translationDelta))
    (:NewEnumerator1
      (Transformation|AddActorLocalOffset translationDelta false false))))

(fn RotationDeltaReceived
  (params (Delta :type Rotator))
  (Class|Actor|AddActorWorldRotation Delta))

(fn ScaleDeltaReceived
  (params (delta :type Vector))
  (bind _returnvalue (* delta 0.02))
  (bind _returnvalue_2 (Transformation|GetActorScale3D))
  (bind _returnvalue_3 (+ _returnvalue _returnvalue_2))
  (if (Math|Float|InRange(Float) (.X (Math|Vector|BreakVector _returnvalue_3)) (Variables|Default|GetminScale) (Variables|Default|GetmaxScale))
    (Transformation|SetActorScale3D _returnvalue_3)))

(fn IsHovered
  (return false))

(fn IsSelected
  (return false))