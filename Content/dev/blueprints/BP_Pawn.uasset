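; Mouse-driven camera pawn for orbiting, panning and zooming around a scene and its selectable objects.
; Left-drag rotates unless the GameState transform gizmo is dragging, and right-drag pans.
; Tick optionally clamps pitch and interpolates spring arm length toward the wheel-set target.
; FocusToActor (object under cursor) and FrameSelected (selected BP_SelectableObject) glide the spring arm there via timeline, then set CineCamera focus tracking.
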(event Custom|LimitCamera
  (bind _returnvalue (Transformation|GetActorRotation))
  (bind _ylimitmin (Variables|Default|GetYLimitMin))
  (bind _ylimitmax (Variables|Default|GetYLimitMax))
  (bind (_roll _pitch _yaw) (Math|Rotator|BreakRotator _returnvalue))
  (bind _returnvalue_2 (< _pitch _ylimitmin))
  ;[1 1 1] camera limit
  (if (Variables|Default|GetrotationYlimit)
    (if (or _returnvalue_2 (> _pitch _ylimitmax))
      (Transformation|SetActorRotation (Math|Rotator|MakeRotator 0.0 (Math|Float|SelectFloat _ylimitmin _ylimitmax _returnvalue_2) _yaw)))))

(event Custom|Focus%20to%20the%20item
  (params (Actor :type Actor%20Object%20Reference))
  ;[1 1 1] focus on actor
  (bind _output_get (Variables|Default|SetFocusedItem Actor)) ; Set focused item
  (Utilities|IsValid _output_get
    (:Is%20Valid
      (bind _lerp (Timeline|Timeline_1 PlayFromStart)
        (:Update
          (Transformation|SetWorldLocation (Variables|Default|GetSpringArm) (Math|Vector|Lerp(Vector) (Transformation|GetActorLocation) (+ (Transformation|GetActorLocation (Variables|Default|GetFocusedItem)) "0, 0,100.000000") _lerp) false false))
        (:Finished
          (CallFunction|SetCameraFocusActor (Variables|Default|GetFocusedItem)))))))

(event Custom|Set%20Camera%20Focus%20Actor
  (params (actor :type Actor%20Object%20Reference))
  ;[1 1 1] focus on actor
  (Variables|/Script/CinematicCamera.CineCameraComponent|SetFocusSettings (Variables|Default|GetCineCamera) (Utilities|Struct|MakeCameraFocusSettings "Tracking" 1e+05 (Utilities|Struct|MakeCameraTrackingFocusSettings (Utilities|ResolveSoftReference actor) "0.000000,0.000000,0.000000" false) true 1.0)))

(event EventBeginPlay
  ;[1 1 1] BeginPlay
  (Variables|/Script/Engine.PlayerController|SetbShowMouseCursor (Game|GetPlayerController 0) true)
  (bind _asbp_game_state (Utilities|Casting|CastToBP_GameState (Game|GetGameState)))
  (Variables|Default|SetGameState _asbp_game_state))

(event EventTick
  (params (DeltaSeconds :type Float%20%28single-precision%29))
  ;[1 1 1] event tick
  (CallFunction|LimitCamera)
  (CallFunction|HandleZoom (Variables|Default|GetzoomInterpSpeed)))

(event Input|ActionEvents|InputActionFocusToActor
  (params (Key :type Key%20Structure :default "None"))
  (bind _returnvalue (Game|GetPlayerController 0))
  (bind _array (Utilities|Array|MakeArray "ObjectTypeQuery1" "ObjectTypeQuery2" "ObjectTypeQuery7"))
  (bind (_hitresult _returnvalue_2) (Class|PlayerController|GetHitResultUnderCursorforObjects _returnvalue _array false))
  ;[1 1 1] focus on actor
  (:Pressed
    (if _returnvalue_2
      (CallFunction|FocustotheItem (.HitActor (Collision|BreakHitResult _hitresult))))))

(event Input|ActionEvents|InputActionFrameSelected
  (params (Key :type Key%20Structure :default "None"))
  ;[1 1 1] focus on actor
  (:Pressed
    (CallFunction|FocusSelectedItem)))

(event Input|MouseEvents|MouseX
  (params (AxisValue :type Float%20%28single-precision%29))
  ;[1 1 1] Move Camera Around
  (if (and (not (.bGizmoDragging (Utilities|Struct|BreakTransformState (Variables|/Game/dev/blueprints/BP_GameState.BP_GameState_C|GetTransformation (Variables|Default|GetGameState))))) (Game|Player|IsInputKeyDown (Game|GetPlayerController 0) "LeftMouseButton"))
    (Class|Actor|AddActorWorldRotation (Math|Rotator|MakeRotator 0.0 0.0 (* AxisValue (Variables|Default|GetrotationSpeed))))
    (elif (Game|Player|IsInputKeyDown (Game|GetPlayerController 0) "RightMouseButton")
      (Transformation|AddActorLocalOffset (Math|Vector|MakeVector 0.0 (* (* -1 AxisValue) (Variables|Default|GetpanSpeed)) 0.0) false false))))

(event Input|MouseEvents|MouseY
  (params (AxisValue :type Float%20%28single-precision%29))
  ;[1 1 1] Move Camera Around
  (if (and (not (.bGizmoDragging (Utilities|Struct|BreakTransformState (Variables|/Game/dev/blueprints/BP_GameState.BP_GameState_C|GetTransformation (Variables|Default|GetGameState))))) (Game|Player|IsInputKeyDown (Game|GetPlayerController 0) "LeftMouseButton"))
    (Transformation|AddActorLocalRotation (Math|Rotator|MakeRotator 0.0 (* AxisValue (Variables|Default|GetrotationSpeed)) 0.0) false false)
    (elif (Game|Player|IsInputKeyDown (Game|GetPlayerController 0) "RightMouseButton")
      (Transformation|AddActorLocalOffset (Math|Vector|MakeVector 0.0 0.0 (* (* -1 AxisValue) (Variables|Default|GetpanSpeed))) false false))))

(event Input|MouseEvents|MouseWheelUp
  (params (Key :type Key%20Structure :default "None"))
  ;[1 1 1] zoom in/out
  (:Pressed
    (Variables|Default|SettargetArmLengthValue (- (Variables|Default|GettargetArmLengthValue) (Variables|Default|GetzoomStep)))))

(event Input|MouseEvents|MouseWheelDown
  (params (Key :type Key%20Structure :default "None"))
  ;[1 1 1] zoom in/out
  (:Pressed
    (Variables|Default|SettargetArmLengthValue (+ (Variables|Default|GettargetArmLengthValue) (Variables|Default|GetzoomStep)))))

(fn ConstructionScript)

(fn HandleZoom
  (params (InterpSpeed :type Float%20%28single-precision%29))
  (Variables|/Script/Engine.SpringArmComponent|SetTargetArmLength (Variables|Default|GetSpringArm) (Math|Interpolation|FInterpTo (Variables|/Script/Engine.SpringArmComponent|GetTargetArmLength (Variables|Default|GetSpringArm)) (Variables|Default|GettargetArmLengthValue) (Utilities|Time|GetWorldDeltaSeconds) InterpSpeed)))

(fn FocusSelectedItem
  (LocalVariables|SetSelectedObject 0)
  (bind _outactors (Actor|GetAllActorsOfClass "/Game/dev/blueprints/BP_SelectableObject.BP_SelectableObject_C"))
  (for _array_element _outactors
    (if (Variables|/Game/dev/blueprints/BP_SelectableObject.BP_SelectableObject_C|GetbSelected _array_element)
      (LocalVariables|SetSelectedObject _array_element)))
  (bind _selectedobject (LocalVariables|GetSelectedObject)
    (:then
      (CallFunction|FocustotheItem _selectedobject))
    (:else)))