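; BP_GizmoUtils is a set of helper functions for transform gizmos, covering grid snapping and initial placement.
; The vector and rotator snap functions apply GridSnapFloat to each component with one shared grid size and return the three values separately.
; The initial gizmo transform takes the owner's location and GizmoScale, with zero rotation in World space or the owner's rotation in Local space.
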(fn SnapVectortoGrid
  (params (gridSize :type Float%20%28single-precision%29) (in :type Vector))
  (return (Math|Vector|MakeVector (Math|Float|SnapToGrid(Float) (.x in) gridSize) (Math|Float|SnapToGrid(Float) (.y in) gridSize) (Math|Float|SnapToGrid(Float) (.z in) gridSize))))

(fn SnapRotatortoGrid
  (params (gridSize :type Float%20%28single-precision%29) (in :type Rotator))
  (return (Math|Rotator|MakeRotator (Math|Float|SnapToGrid(Float) (.roll in) gridSize) (Math|Float|SnapToGrid(Float) (.pitch in) gridSize) (Math|Float|SnapToGrid(Float) (.yaw in) gridSize))))

(fn GetInitialTransformforGizmo
  (params (space :type ETransformationSpace%20Enum :default "NewEnumerator0") (owner :type BP%20Selectable%20Object%20Object%20Reference))
  (return (Math|Transform|MakeTransform (Transformation|GetActorLocation owner) (Utilities|Select :Index space :NewEnumerator0 "0, 0, 0" :NewEnumerator1 (Transformation|GetActorRotation owner)) (Math|Conversions|ToVector(Float) (Variables|/Game/dev/blueprints/BP_SelectableObject.BP_SelectableObject_C|GetgizmoScale owner)))))