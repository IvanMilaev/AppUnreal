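; BP_Configurator handles JSON commands from a web client to switch variants and change the render resolution at runtime.
; OnReceiveCommand routes on the "command" field, either activating a named variant through the Variant Manager's level variant sets or changing resolution.
; Resolution changes pass size and aspect-ratio checks, run r.setres, then resize BP_Pawn's CineCamera filmback to the new aspect, keeping the shorter sensor side at FilmBackSensorSize.
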(event Custom|OnReceiveCommand
  (params (json :type Blueprint%20Json%20Object%20Structure))
  (bind _returnvalue (Class|BlueprintJsonLibrary|ToJsonValue(JsonObject) json "command"))
  ;[1 1 1] web command handler
  (Variables|Default|SetjsonData json)
  (if (Class|BlueprintJsonLibrary|JsonIsNull _returnvalue)
    (Development|PrintString "json has no key command")
    (else
      (switch string (Class|BlueprintJsonLibrary|ToString(JsonValue) _returnvalue)
        (:variant
          (CallFunction|ToggleVariantManagerOption))
        (:changeResolution
          (CallFunction|ChangeResolution))))))

(event Custom|toggleVariantManagerOption
  (bind _jsondata (Variables|Default|GetjsonData))
  (bind _returnvalue (Class|BlueprintJsonLibrary|ToJsonValue(JsonObject) _jsondata "item"))
  (bind _returnvalue_2 (Class|BlueprintJsonLibrary|ToJsonValue(JsonObject) _jsondata "value"))
  ;[1 1 1] handle variant manager option change
  (if (or (Class|BlueprintJsonLibrary|JsonIsNull _returnvalue) (Class|BlueprintJsonLibrary|JsonIsNull _returnvalue_2))
    (Development|PrintString "invalid json for variant manager" true true "(R=0.718000,G=0.000000,B=0.024921,A=1.000000)")
    (else
      (bind _returnvalue_3 (Class|LevelVariantSetsActor|GetLevelVariantSets (Variables|Default|GetvariantManager) true))
      (Class|Variant|Switchon (Class|VariantSet|GetVariantbyName (Class|LevelVariantSets|GetVariantSetbyName _returnvalue_3 (Class|BlueprintJsonLibrary|ToString(JsonValue) _returnvalue)) (Class|BlueprintJsonLibrary|ToString(JsonValue) _returnvalue_2))))))

(event Custom|ChangeResolution
  (bind _jsondata (Variables|Default|GetjsonData))
  (bind _returnvalue (Class|BlueprintJsonLibrary|ToJsonValue(JsonObject) _jsondata "width"))
  (bind _returnvalue_2 (Class|BlueprintJsonLibrary|ToJsonValue(JsonObject) _jsondata "height"))
  (bind _returnvalue_3 (Class|BlueprintJsonLibrary|ToFloat(JsonValue) _returnvalue_2))
  (bind _returnvalue_4 (Class|BlueprintJsonLibrary|ToFloat(JsonValue) _returnvalue))
  ;[1 1 1] change Resolution
  (if (or (Class|BlueprintJsonLibrary|JsonIsNull _returnvalue) (Class|BlueprintJsonLibrary|JsonIsNull _returnvalue_2))
    (Development|PrintString "invalid json for change resolution" true true "(R=0.718000,G=0.000000,B=0.024921,A=1.000000)")
    (else
      (bind _out (CallFunction|CheckResolutionSettings _returnvalue_4 _returnvalue_3))
      (if _out
        (Development|ExecuteConsoleCommand (Utilities|String|ToString(Text) (Utilities|Text|FormatText "r.setres {width}x{height}w" (Class|BlueprintJsonLibrary|ToString(JsonValue) _returnvalue) (Class|BlueprintJsonLibrary|ToString(JsonValue) _returnvalue_2))) 0)
        (bind _asbp_pawn (Utilities|Casting|CastToBP_Pawn (Game|Player|GetPlayerPawn 0)))
        (if (Utilities|IsValid (Actor|GetComponentbyClass _asbp_pawn "/Script/CinematicCamera.CineCameraComponent"))
          (bind (_sensorwidth _sensorheight) (CallFunction|ComputeCameraSensorWidthHeight _returnvalue_4 _returnvalue_3))
          (Variables|/Script/CinematicCamera.CineCameraComponent|SetFilmback (Actor|GetComponentbyClass _asbp_pawn "/Script/CinematicCamera.CineCameraComponent") (Utilities|Struct|MakeCameraFilmbackSettings _sensorwidth _sensorheight))
          (else
            (Development|PrintString "cine camera component not found" true true "(R=0.723958,G=0.000000,B=0.000000,A=1.000000)")))
        (else
          (Development|PrintString "invalid width height values" true true "(R=0.593750,G=0.000000,B=0.056047,A=1.000000)"))))))

(fn ConstructionScript)

(fn CheckResolutionSettings
  (params (width :type Float%20%28single-precision%29) (height :type Float%20%28single-precision%29))
  (return (and (Math|Float|InRange(Float) (/ width height) 0.2 5.0) (and (> width 2e+01) (> height 2e+01)))))

(fn ComputeCameraSensorWidthHeight
  (params (width :type Float%20%28single-precision%29) (height :type Float%20%28single-precision%29))
  (bind _filmbacksensorsize (LocalVariables|GetfilmBackSensorSize))
  (bind _filmbacksensorsize_2 (LocalVariables|GetfilmBackSensorSize))
  (if (> width height)
    (LocalVariables|SetsWidth (* (/ width height) _filmbacksensorsize_2))
    (bind _output_get (LocalVariables|SetsHeight _filmbacksensorsize_2))
    (else
      (LocalVariables|SetsHeight (* (/ height width) _filmbacksensorsize))
      (bind _output_get_2 (LocalVariables|SetsWidth _filmbacksensorsize))))
  (return _output_get_2 _output_get))