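; BP_Renderer renders a high-resolution PNG still from the player's camera at runtime through Movie Render Queue.
; It copies the BP_Pawn cine camera's lens settings to its Camera and moves TransformActor to that camera's transform.
; It then replaces queued jobs with a one-frame deferred-pass job on the target sequence and map, tiled by resolution.
; An in-process executor renders it in the current level with an overlay widget.
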(event EventBeginPlay)

(event Collision|EventActorBeginOverlap
  (params (OtherActor :type Actor%20Object%20Reference)))

(event EventTick
  (params (DeltaSeconds :type Float%20%28single-precision%29)))

(fn ConstructionScript)

(fn MakeRenderfromPlayerCamera
  (params (ResolutionX :type Integer) (ResolutionY :type Integer) (FileName :type String))
  (bind _returnvalue (|MoviePipelineQueueEngineSubsystem))
  (CallFunction|SyncRenderCameraWidthPlayerCamera)
  (CallFunction|ClearAllJobs)
  (bind _returnvalue_2 (Class|MoviePipelineQueue|AllocateNewJob (Class|MoviePipelineQueueEngineSubsystem|GetQueue (|MoviePipelineQueueEngineSubsystem)) "/Script/MovieRenderPipelineCore.MoviePipelineExecutorJob"))
  (Variables|/Script/MovieRenderPipelineCore.MoviePipelineExecutorJob|SetSequence _returnvalue_2 (Variables|Default|GetTargetSequence))
  (Variables|/Script/MovieRenderPipelineCore.MoviePipelineExecutorJob|SetMap _returnvalue_2 (Variables|Default|GettargetMap))
  (Utilities|FlowControl|Sequence
    (:then_0
      (bind _returnvalue_3 (Class|MoviePipelineConfigBase|FindorAddSettingbyClass (Class|MoviePipelineExecutorJob|GetConfiguration _returnvalue_2) "/Script/MovieRenderPipelineCore.MoviePipelineOutputSetting" false))
      (Variables|/Script/MovieRenderPipelineCore.MoviePipelineOutputSetting|SetCustomStartFrame _returnvalue_3 0)
      (Variables|/Script/MovieRenderPipelineCore.MoviePipelineOutputSetting|SetCustomEndFrame _returnvalue_3 1))
    (:then_1
      (Class|MoviePipelineConfigBase|FindorAddSettingbyClass (Class|MoviePipelineExecutorJob|GetConfiguration _returnvalue_2) "/Script/MovieRenderPipelineRenderPasses.MoviePipelineImageSequenceOutput_PNG" false))
    (:then_2
      (bind _returnvalue_4 (Class|MoviePipelineConfigBase|FindorAddSettingbyClass (Class|MoviePipelineExecutorJob|GetConfiguration _returnvalue_2) "/Script/MovieRenderPipelineCore.MoviePipelineOutputSetting" false))
      (Variables|/Script/MovieRenderPipelineCore.MoviePipelineOutputSetting|SetOutputResolution _returnvalue_4 (Utilities|Struct|MakeIntPoint ResolutionX ResolutionY))
      (Variables|/Script/MovieRenderPipelineCore.MoviePipelineOutputSetting|SetFileNameFormat _returnvalue_4 FileName))
    (:then_3
      (Class|MoviePipelineConfigBase|FindorAddSettingbyClass (Class|MoviePipelineExecutorJob|GetConfiguration _returnvalue_2) "/Script/MovieRenderPipelineRenderPasses.MoviePipelineDeferredPassBase" false))
    (:then_4
      (bind _returnvalue_5 (Class|MoviePipelineConfigBase|FindorAddSettingbyClass (Class|MoviePipelineExecutorJob|GetConfiguration _returnvalue_2) "/Script/MovieRenderPipelineCore.MoviePipelineHighResSetting" false))
      (Variables|/Script/MovieRenderPipelineCore.MoviePipelineHighResSetting|SetTileCount _returnvalue_5 (Math|Integer|Clamp(Integer) (/ (Math|Integer|Max(Integer) ResolutionX ResolutionY) 1024) 1 100))
      (Variables|/Script/MovieRenderPipelineCore.MoviePipelineHighResSetting|SetOverlapRatio _returnvalue_5 0.05))
    (:then_5
      (bind _returnvalue_6 (Game|ConstructObjectfromClass "/Script/MovieRenderPipelineCore.MoviePipelineInProcessExecutor" _returnvalue))
      (Utilities|FlowControl|Sequence
        (:then_0
          (Variables|/Script/MovieRenderPipelineCore.MoviePipelineInProcessExecutor|SetbUseCurrentLevel _returnvalue_6 true))
        (:then_1
          (Variables|/Script/MovieRenderPipelineCore.MoviePipelineExecutorBase|SetDebugWidgetClass _returnvalue_6 "/MovieRenderPipeline/Blueprints/UI_MovieRenderPipelineScreenOverlay.UI_MovieRenderPipelineScreenOverlay_C"))
        (:then_2
          (Class|MoviePipelineQueueEngineSubsystem|RenderQueuewithExecutorInstance _returnvalue _returnvalue_6)
          (return _returnvalue_6))))))

(fn ClearAllJobs
  (bind _returnvalue (|MoviePipelineQueueEngineSubsystem))
  (bind _returnvalue_2 (Class|MoviePipelineQueueEngineSubsystem|GetQueue _returnvalue))
  (for _array_element (Class|MoviePipelineQueue|GetJobs _returnvalue_2)
    (Class|MoviePipelineQueue|DeleteJob _returnvalue_2 _array_element))
  (return))

(fn SyncRenderCameraWidthPlayerCamera
  (bind _camera (Variables|Default|Getcamera))
  (bind _returnvalue (Class|CineCameraActor|GetCineCameraComponent _camera))
  (bind _asbp_pawn (Utilities|Casting|CastToBP_Pawn (Game|Player|GetPlayerPawn 0)))
  (if (Utilities|IsValid (Actor|GetComponentbyClass _asbp_pawn "/Script/CinematicCamera.CineCameraComponent"))
    (Transformation|SetActorTransform (Variables|Default|GettransformActor) (Transformation|GetWorldTransform (Actor|GetComponentbyClass _asbp_pawn "/Script/CinematicCamera.CineCameraComponent")))
    (Variables|/Script/CinematicCamera.CineCameraComponent|SetFilmback _returnvalue (Variables|/Script/CinematicCamera.CineCameraComponent|GetFilmback (Actor|GetComponentbyClass _asbp_pawn "/Script/CinematicCamera.CineCameraComponent")))
    (Variables|/Script/CinematicCamera.CineCameraComponent|SetFocusSettings _returnvalue (Variables|/Script/CinematicCamera.CineCameraComponent|GetFocusSettings (Actor|GetComponentbyClass _asbp_pawn "/Script/CinematicCamera.CineCameraComponent")))
    (Variables|/Script/CinematicCamera.CineCameraComponent|SetLensSettings _returnvalue (Variables|/Script/CinematicCamera.CineCameraComponent|GetLensSettings (Actor|GetComponentbyClass _asbp_pawn "/Script/CinematicCamera.CineCameraComponent")))
    (Variables|/Script/CinematicCamera.CineCameraComponent|SetCurrentFocalLength _returnvalue (Variables|/Script/CinematicCamera.CineCameraComponent|GetCurrentFocalLength (Actor|GetComponentbyClass _asbp_pawn "/Script/CinematicCamera.CineCameraComponent")))
    (return)
    (else
      (Development|PrintString "there is no cine camera component in player pawn" true true "(R=0.463542,G=0.054572,B=0.017638,A=1.000000)"))))