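; Dev test actor that launches an asset-prep job on a spawned Manager and loads the resulting imported level.
; Pressing 1 calls the Manager's Test, then a looping timer polls its status until the job first completes.
; With the editor, it registers a content mount point; otherwise it mounts an external pak, then opens the level on success.
; Paths are hardcoded, and StartAssetPrepServer is a stub returning false.
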(event Custom|checkAssetPrep
  (bind _returnvalue (Utilities|String|MakeLiteralString "ImportTemp"))
  (bind _returnvalue_2 (Utilities|String|MakeLiteralString "AutomatedImport"))
  (bind _returnvalue_3 (Utilities|String|MakeLiteralString "AutomatedImport"))
  (bind _returnvalue_4 (Utilities|String|MakeLiteralString "ImportTemp"))
  (bind _returnvalue_5 (Utilities|String|MakeLiteralString "d:/temp"))
  (bind _returnvalue_6 (Utilities|String|MakeLiteralString "d:/temp"))
  (bind _returnvalue_7 (Utilities|String|Append "/Game/" _returnvalue))
  (bind _returnvalue_8 (Utilities|String|Append "/" _returnvalue_3 "/editor/content/" _returnvalue_4))
  (bind _returnvalue_9 (Utilities|String|Append _returnvalue_6 "/" _returnvalue_2 "/" _returnvalue_2 ".pak"))
  (bind _returnvalue_10 (Utilities|String|Append _returnvalue_5 _returnvalue_8))
  (if (and (Utilities|Enum|Equal(Enum) (Class|Manager|GetCurrentStatus (Variables|Default|GetMAssetManager)) "JobCompleted") (not (Variables|Default|GetjobCompleted)))
    (Development|PrintString "JOB COMPLETED!!!!!" true true "(R=0.000000,G=1.000000,B=0.036073,A=1.000000)" 1e+01)
    (Variables|Default|SetjobCompleted true)
    (if (Class|HotLoadBPLibraryUtils|IswithEditor)
      (Development|PrintString "with editor")
      (if (Class|HotLoadBPLibraryUtils|IswithEditor)
        (Development|PrintString (Utilities|String|Append "Register Editor " _returnvalue_7 " " _returnvalue_10))
        (if (Class|HotLoadBPLibraryUtils|RegisterMountPoint _returnvalue_7 _returnvalue_10)
          (Game|OpenLevel(byName) (Utilities|String|StringToName (Utilities|String|Append "/Game/" (Utilities|String|MakeLiteralString "ImportTemp") "/" (Utilities|String|MakeLiteralString "AutomatedImport"))) :!label _label)))
      (else
        (Development|PrintString (Utilities|String|Append "Register Runtime " _returnvalue_9 " " "/Game/"))
        (if (Class|HotLoadBPLibraryUtils|MountExternalPak _returnvalue_9 "/Game/")
          (goto _label))))))

(event EventBeginPlay
  (Input|EnableInput (Game|GetPlayerController 0))
  (bind _returnvalue (Game|SpawnActorfromClass "/Script/AssetManager_DDDSource.Manager" (Math|Transform|MakeTransform "0, 0, 0") "Undefined" 0 0))
  (Variables|Default|SetMAssetManager _returnvalue))

(event Collision|EventActorBeginOverlap
  (params (OtherActor :type Actor%20Object%20Reference)))

(event EventTick
  (params (DeltaSeconds :type Float%20%28single-precision%29)))

(event Input|KeyboardEvents|1
  (params (Key :type Key%20Structure :default "None"))
  (:Pressed
    (bind _returnvalue (Class|Manager|Test (Variables|Default|GetMAssetManager)))
    (Development|PrintString "test launched")
    (if _returnvalue
      (Utilities|Time|SetTimerbyEvent (delegate Custom|checkAssetPrep) 1.0 true))))

(fn ConstructionScript)

(fn StartAssetPrepServer
  (params (JobDescription :type String) (IPAddress :type String) (Port :type Integer))
  (return false))